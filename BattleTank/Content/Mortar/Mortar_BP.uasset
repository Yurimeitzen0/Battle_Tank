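; Mortar Blueprint for an aiming emplacement with a barrel, a dome turret and an on-screen health bar widget.
; On BeginPlay it initialises its TankAiming component with the barrel and the dome as the turret.
; It then casts the widget component's user widget to HealthBar2 and hands it a reference to itself as the controlled tank.
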(event EventBeginPlay
  (Class|TankAimingComponent|Initialise (Variables|Default|GetTankAiming_0) (Variables|Default|GetBarrel) (Variables|Default|GetDome))
  (CallFunction|InitialiseHealth))

(fn ConstructionScript)

(fn InitialiseHealth
  (bind _ashealth_bar_2 (Utilities|Casting|CastToHealthBar2 (UserInterface|GetUserWidgetObject (Variables|Default|GetWidget))))
  (Variables|/Game/UI/HealthBar2.HealthBar2_C|SetgetControlledTank2 _ashealth_bar_2 self))